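; Melee knife weapon for the first-person pawn, with stats set in the construction script and saved to the pawn's MeleeWeapon on Unequip.
; Fire plays one of three random arm montages, then runs a short camera trace that calls Jahae on any AIPawn_BP hit.
; The trace result places a knife decal, oriented differently for upward-facing surfaces.
; A single-round ammo count, refilled after a retriggerable delay, acts as the attack cooldown.
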(event EventUnequip
  (Variables|/Game/FPSPawn/Blueprints/FPSPawn_BP.FPSPawn_BP_C|SetMeleeWeapon (.AsFPSPawn%20BP (Utilities|Casting|CastToFPSPawn_BP (Game|GetPlayerCharacter 0))) (Utilities|Struct|MakeGunData "NewEnumerator4" "Weapon_Knife_C" (Variables|Default|GetAmmoCnt) (Variables|Default|GetAmmoMax) (Variables|Default|GetReloadTime) (Variables|Default|GetBulletSpread))))

(event EventFire
  (bind _returnvalue (Game|GetPlayerCharacter 0))
  (bind _asfpspawn_bp (Utilities|Casting|CastToFPSPawn_BP _returnvalue))
  (bind _mesh1p (Variables|/Game/FPSPawn/Blueprints/FPSPawn_BP.FPSPawn_BP_C|GetMesh1P _asfpspawn_bp))
  (if (> (Variables|Default|GetAmmoCnt) 0)
    (Utilities|FlowControl|Sequence
      (:then_0
        (Math|Integer|DecrementInt (Variables|Default|GetAmmoCnt)
          (:%20%20
            (switch int (Math|Random|RandomIntegerinRange 0 2)
              (:0
                (Animation|Montage|PlayMontage _mesh1p "/Game/FPSPawn/Animations/Montages/Arms_Knife_Attack_01_anim_Montage.Arms_Knife_Attack_01_anim_Montage"))
              (:1
                (Animation|Montage|PlayMontage _mesh1p "/Game/FPSPawn/Animations/Montages/Arms_Knife_Attack_02_anim_Montage.Arms_Knife_Attack_02_anim_Montage"))
              (:2
                (Animation|Montage|PlayMontage _mesh1p "/Game/FPSPawn/Animations/Montages/Arms_Knife_Attack_03_anim_Montage.Arms_Knife_Attack_03_anim_Montage"))))))
      (:then_1
        (bind (_impactnormal _impactpoint) (CallFunction|LineTrace))
        (CallFunction|SpawnDecalTracer _impactnormal _impactpoint))
      (:then_2
        (Utilities|FlowControl|RetriggerableDelay (Variables|Default|GetReloadTime))
        (Variables|Default|SetAmmoCnt (Variables|Default|GetAmmoMax))))))

(fn ConstructionScript
  (|CallParentFunction)
  (Variables|Default|SetAmmoMax 1)
  (Variables|Default|SetAmmoCnt 1)
  (Variables|Default|SetReloadTime 0.2)
  (Variables|Default|SetBulletSpread 0.0)
  (Variables|Default|SetName "NewEnumerator4")
  (Variables|Default|SetAutoAvailable false)
  (Variables|Default|SetDamage 5e+01)
  (Variables|Default|SetRotationOffset "0, 0, 0"))

(fn LineTrace
  (bind _returnvalue (Game|GetPlayerCharacter 0))
  (bind _bulletspread (Variables|Default|GetBulletSpread))
  (bind _returnvalue_2 (* _bulletspread -1.0))
  (bind _asfpspawn_bp (Utilities|Casting|CastToFPSPawn_BP _returnvalue))
  (bind _firstpersoncamera (Variables|/Game/FPSPawn/Blueprints/FPSPawn_BP.FPSPawn_BP_C|GetFirstPersonCamera _asfpspawn_bp))
  (bind _returnvalue_3 (Transformation|GetWorldLocation _firstpersoncamera))
  (bind (_outhit _returnvalue_4) (Collision|LineTraceByChannel (+ _returnvalue_3 (Variables|Default|GetAimOffset)) (+ (+ _returnvalue_3 (* (Math|Vector|GetForwardVector _firstpersoncamera) 2e+02)) (Math|Vector|MakeVector (Math|Random|RandomFloatinRange _returnvalue_2 _bulletspread) (Math|Random|RandomFloatinRange _returnvalue_2 _bulletspread) (Math|Random|RandomFloatinRange _returnvalue_2 _bulletspread))) "TraceTypeQuery1" false 0 "None")) ; CameraShot
  (if _returnvalue_4
    (if (.bSuccess (Utilities|Casting|CastToAIPawn_BP (.HitActor (Collision|BreakHitResult _outhit))))
      (Default|Jahae (.AsAIPawn%20BP (Utilities|Casting|CastToAIPawn_BP (.HitActor (Collision|BreakHitResult _outhit))))))
    (return (.ImpactNormal (Collision|BreakHitResult _outhit)) (.ImpactPoint (Collision|BreakHitResult _outhit)))))

(fn SpawnDecalTracer
  (params (ImpactNormal :type Vector) (ImpactPoint :type Vector))
  (bind _returnvalue (Math|Conversions|RotationFromXVector ImpactNormal))
  (bind _returnvalue_2 (Game|GetPlayerCharacter 0))
  (bind _asfpspawn_bp (Utilities|Casting|CastToFPSPawn_BP _returnvalue_2))
  (bind _firstpersoncamera (Variables|/Game/FPSPawn/Blueprints/FPSPawn_BP.FPSPawn_BP_C|GetFirstPersonCamera _asfpspawn_bp))
  (if (Math|Vector|Equal(Vector) ImpactNormal "0, 0,1.000000" 0.0001)
    (Game|SpawnActorfromClass "/Game/FPSPawn/Animations/Montages/KnifeDecal_BP.KnifeDecal_BP_C" (Math|Transform|MakeTransform ImpactPoint (Math|Rotator|MakeRotator -9e+01 9e+01 (.yaw (Math|Conversions|RotationFromXVector (Math|Vector|GetForwardVector _firstpersoncamera)))) "1.000000,0.300000,0.300000") "Undefined" 0 0)
    (else
      (Game|SpawnActorfromClass "/Game/FPSPawn/Animations/Montages/KnifeDecal_BP.KnifeDecal_BP_C" (Math|Transform|MakeTransform ImpactPoint (Math|Rotator|MakeRotator (+ (.roll (Transformation|GetWorldRotation _firstpersoncamera)) 9e+01) (.pitch _returnvalue) (+ (.yaw _returnvalue) 1e+03)) "1.000000,0.300000,0.300000") "Undefined" 0 0))))