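; MP5 weapon for the first-person pawn, with semi and full-auto fire, timed montage reload and saved state on unequip.
; The construction script sets its stats; full-auto loops through a delayed gate with recoil growing per bullet.
; Each shot runs a spread-randomized camera trace that triggers AI hits, then spawns decals, random tracers and muzzle flash.
; ADS timelines blend FOV and arm position and change spread, only while the character is falling.
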(event EventUnequip
  (bind _returnvalue (Game|GetPlayerCharacter 0))
  (bind _asfpspawn_bp (Utilities|Casting|CastToFPSPawn_BP _returnvalue))
  (bind _weapontoequip (Variables|/Game/FPSPawn/Blueprints/FPSPawn_BP.FPSPawn_BP_C|GetWeaponToEquip _asfpspawn_bp))
  (if (not (== (Variables|/Game/FPSPawn/Blueprints/FPSPawn_BP.FPSPawn_BP_C|GetWeaponEquipped _asfpspawn_bp) _weapontoequip))
    (switch int _weapontoequip
      (:1
        (Variables|/Game/FPSPawn/Blueprints/FPSPawn_BP.FPSPawn_BP_C|SetMain2Weapon _asfpspawn_bp (Utilities|Struct|MakeGunData "NewEnumerator3" "Weapon_MP5_C" (Variables|Default|GetAmmoCnt) (Variables|Default|GetAmmoMax) (Variables|Default|GetReloadTime) (Variables|Default|GetBulletSpread))))
      (:2
        (Variables|/Game/FPSPawn/Blueprints/FPSPawn_BP.FPSPawn_BP_C|SetMain1Weapon _asfpspawn_bp (Utilities|Struct|MakeGunData "NewEnumerator3" "Weapon_MP5_C" (Variables|Default|GetAmmoCnt) (Variables|Default|GetAmmoMax) (Variables|Default|GetReloadTime) (Variables|Default|GetBulletSpread)))))))

(event EventStopFiring
  (Variables|Default|SetFiredBullets -1)
  (Utilities|FlowControl|Gate true) ; enters at Close
)

(event EventADS
  (params (Toggle :type Boolean))
  (bind _returnvalue (Game|GetPlayerCharacter 0))
  (bind _asfpspawn_bp (Utilities|Casting|CastToFPSPawn_BP _returnvalue))
  (bind _firstpersoncamera (Variables|/Game/FPSPawn/Blueprints/FPSPawn_BP.FPSPawn_BP_C|GetFirstPersonCamera _asfpspawn_bp))
  (bind _mesh1p (Variables|/Game/FPSPawn/Blueprints/FPSPawn_BP.FPSPawn_BP_C|GetMesh1P _asfpspawn_bp))
  (if (AI|Components|NavMovement|IsFalling (Variables|/Script/Engine.Character|GetCharacterMovement (.AsFPSPawn%20BP (Utilities|Casting|CastToFPSPawn_BP (Game|GetPlayerCharacter 0)))))
    (if Toggle
      (bind _float (Timeline|Timeline_0 Play)
        (:Update
          (Camera|SetFieldOfView _firstpersoncamera (Math|Float|Lerp 9e+01 45.0 _float))
          (Transformation|SetRelativeTransform _mesh1p (Math|Transform|MakeTransform (Math|Vector|Lerp(Vector) "1.600000,7.800000,-23.677500" "0.000000, 0,-16.500000" _float) "1.000000,-1.100000, 0" "1,1,1") false false)
          (Variables|Default|SetBulletSpread 5e+01)))
      (else
        (bind _float_2 (Timeline|Timeline_1 Play)
          (:Update
            (Camera|SetFieldOfView _firstpersoncamera (Math|Float|Lerp 45.0 9e+01 _float_2))
            (Transformation|SetRelativeTransform _mesh1p (Math|Transform|MakeTransform (Math|Vector|Lerp(Vector) "0.000000,0.000000,-16.500000" "1.600000,7.800000,-23.677500" _float_2) "0, 0, 0" "1,1,1") false false)
            (Variables|Default|SetBulletSpread 1e+02)))))))

(event EventReload
  (bind _returnvalue (Game|GetPlayerCharacter 0))
  (bind _asfpspawn_bp (Utilities|Casting|CastToFPSPawn_BP _returnvalue))
  (if (< (Variables|Default|GetAmmoCnt) (Variables|Default|GetAmmoMax))
    (Utilities|FlowControl|DoOnce false :!label _label
      (:Completed
        (Variables|/Game/FPSPawn/Blueprints/FPSPawn_BP.FPSPawn_BP_C|SetIsReloading _asfpspawn_bp true)
        (Animation|Montage|MontagePlay (Components|SkeletalMesh|GetAnimInstance (Variables|/Game/FPSPawn/Blueprints/FPSPawn_BP.FPSPawn_BP_C|GetMesh1P _asfpspawn_bp)) "/Game/FPSPawn/Animations/Montages/Arms_MP5_Reload_anim_Montage.Arms_MP5_Reload_anim_Montage" 1.0 "MontageLength" 0.0 true)
        (Components|Animation|PlayAnimation (Variables|Default|GetPrimaryWeapon) "/Game/FPSPawn/Animations/Montages/MP5_Reload_anim_Montage.MP5_Reload_anim_Montage" true)
        (Utilities|FlowControl|Delay (Variables|Default|GetReloadTime))
        (Variables|Default|SetAmmoCnt (Variables|Default|GetAmmoMax))
        (Variables|/Game/FPSPawn/Blueprints/FPSPawn_BP.FPSPawn_BP_C|SetIsReloading _asfpspawn_bp false)
        (goto _label Reset)))))

(event EventFire
  (switch int (Variables|Default|GetFireMode)
    (:0
      (Utilities|Shot)
      (CallFunction|SemiAutoRecoil))
    (:2
      (Utilities|FlowControl|Sequence
        (:then_0
          (goto _label Open))
        (:then_1
          (Utilities|FlowControl|Gate true :!label _label
            (:Exit
              (Utilities|FlowControl|Sequence
                (:then_0
                  (Utilities|Shot)
                  (CallFunction|FullAutoRecoil))
                (:then_1
                  (Utilities|FlowControl|RetriggerableDelay (Variables|Default|GetAutoDelay))
                  (goto _label))))))))))

(fn ConstructionScript
  (|CallParentFunction)
  (Variables|Default|SetAmmoMax 30)
  (Variables|Default|SetAmmoCnt 30)
  (Variables|Default|SetReloadTime 2.0)
  (Variables|Default|SetBulletSpread 5e+01)
  (Variables|Default|SetRotationOffset "1.000000,-1.100000, 0")
  (Variables|Default|SetName "NewEnumerator3")
  (Variables|Default|SetAutoAvailable true)
  (Variables|Default|SetBurstAvailable false)
  (Variables|Default|SetDamage 19.0)
  (Variables|Default|SetAutoDelay 0.08)
  (Variables|Default|SetBurstDelay 0.05)
  (Variables|Default|SetBurstShotNum 3)
  (Variables|Default|SetRecoilPitch -0.3)
  (Variables|Default|SetRecoilYaw -0.2)
  (Variables|Default|SetMuzzleFlash 0.2))

(fn AmmoUpdate
  (bind _returnvalue (Math|Random|RandomFloatinRange 0.7 1.2))
  (Math|Integer|DecrementInt (Variables|Default|GetAmmoCnt)
    (:%20%20
      (Audio|PlaySound2D "/Game/FPSPawn/Sounds/Gunshot.Gunshot" (+ _returnvalue -0.2) _returnvalue 0.0 "/Game/FPSPawn/Sounds/Concurrency_AK.Concurrency_AK" 0)
      (Components|Animation|PlayAnimation (Variables|Default|GetPrimaryWeapon) "/Game/FPSPawn/Animations/Weapons/AK_Fire_anim.AK_Fire_anim" false))))

(fn LineTrace
  (bind _returnvalue (Game|GetPlayerCharacter 0))
  (bind _bulletspread (Variables|Default|GetBulletSpread))
  (bind _muzzle (Variables|Default|GetMuzzle))
  (bind _returnvalue_2 (Transformation|GetWorldLocation _muzzle))
  (bind _returnvalue_3 (* _bulletspread -1.0))
  (bind _asfpspawn_bp (Utilities|Casting|CastToFPSPawn_BP _returnvalue))
  (bind _firstpersoncamera (Variables|/Game/FPSPawn/Blueprints/FPSPawn_BP.FPSPawn_BP_C|GetFirstPersonCamera _asfpspawn_bp))
  (bind _returnvalue_4 (Transformation|GetWorldLocation _firstpersoncamera))
  (bind _outhit (Collision|LineTraceByChannel (+ _returnvalue_4 (Variables|Default|GetAimOffset)) (+ (+ _returnvalue_4 (* (Math|Vector|GetForwardVector _firstpersoncamera) 2e+04)) (Math|Vector|MakeVector (Math|Random|RandomFloatinRange _returnvalue_3 _bulletspread) (Math|Random|RandomFloatinRange _returnvalue_3 _bulletspread) (Math|Random|RandomFloatinRange _returnvalue_3 _bulletspread))) "TraceTypeQuery1" false 0 "None")) ; CameraShot
  (Collision|LineTraceByChannel _returnvalue_2 (.ImpactPoint (Collision|BreakHitResult _outhit)) "TraceTypeQuery1" false 0 "None" true "(R=0.160040,G=1.000000,B=0.000000,A=1.000000)") ; GunShot
  (if (.bSuccess (Utilities|Casting|CastToAIPawn_BP (.HitActor (Collision|BreakHitResult _outhit))))
    (Default|Jahae (.AsAIPawn%20BP (Utilities|Casting|CastToAIPawn_BP (.HitActor (Collision|BreakHitResult _outhit))))))
  (return _returnvalue_2 (.ImpactPoint (Collision|BreakHitResult _outhit))))

(fn SpawnDecalTracer
  (params (Location :type Vector) (SpawnTransformLoc :type Vector) (ImpactPoint :type Vector))
  (Game|SpawnActorfromClass "/Game/FPSPawn/Animations/Montages/BulletDecal_BP.BulletDecal_BP_C" (Math|Transform|MakeTransform SpawnTransformLoc (Math|Conversions|RotationFromXVector ImpactPoint) "0.250000,0.250000,0.250000") "Undefined" 0 0)
  (if (>= (Math|Random|RandomIntegerinRange 1 10) 5)
    (Game|SpawnActorfromClass "/Game/FPSPawn/Blueprints/Weapon/TracerRound_BP.TracerRound_BP_C" (Math|Transform|MakeTransform Location (Transformation|GetWorldRotation (Variables|/Game/FPSPawn/Blueprints/FPSPawn_BP.FPSPawn_BP_C|GetFirstPersonCamera (.AsFPSPawn%20BP (Utilities|Casting|CastToFPSPawn_BP (Game|GetPlayerCharacter 0))))) "0.050000,0.050000,0.050000") "Undefined" 0 0))
  (return))

(fn SemiAutoRecoil
  (bind _returnvalue (Game|GetPlayerController 0))
  (bind _recoilpitch (Variables|Default|GetRecoilPitch))
  (bind _recoilyaw (Variables|Default|GetRecoilYaw))
  (Class|PlayerController|AddPitchInput _returnvalue (Math|Random|RandomFloatinRange (* 1.5 _recoilpitch) _recoilpitch))
  (Class|PlayerController|AddYawInput _returnvalue (Math|Random|RandomFloatinRange _recoilyaw (* -1.0 _recoilyaw))))

(fn FullAutoRecoil
  (bind _returnvalue (Game|GetPlayerController 0))
  (bind _result (Math|Integer|IncrementInt (Variables|Default|GetFiredBullets))
    (:%20%20
      (Variables|Default|SetFiredBullets _result)
      (Class|PlayerController|AddPitchInput _returnvalue (Math|Random|RandomFloatinRange (* 1.5 (+ (Variables|Default|GetRecoilPitch) (* (Variables|Default|GetFiredBullets) -0.01))) (+ (Variables|Default|GetRecoilPitch) (* (Variables|Default|GetFiredBullets) -0.01))))
      (Class|PlayerController|AddYawInput _returnvalue (Math|Random|RandomFloatinRange (+ (Variables|Default|GetRecoilYaw) (* (Variables|Default|GetFiredBullets) -0.01)) (* (+ (Variables|Default|GetRecoilYaw) (* (Variables|Default|GetFiredBullets) -0.01)) -1.0))))))