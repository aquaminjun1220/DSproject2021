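; AWP sniper rifle weapon for the FPS pawn, with scoped aiming, firing, reloading using AK animations, and unequipping.
; ADS runs only while the character is falling, using timelines to blend FOV, arm position and spread around the scope HUD.
; Fire briefly unscopes, traces from the camera with spread, calls Jahae on hit AI, spawns decals and random tracers, and adds recoil.
; Unequip saves ammo and stats to the pawn's weapon slot.
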(event EventUnequip
  (bind _returnvalue (Game|GetPlayerCharacter 0))
  (bind _asfpspawn_bp (Utilities|Casting|CastToFPSPawn_BP _returnvalue))
  (bind _weapontoequip (Variables|/Game/FPSPawn/Blueprints/FPSPawn_BP.FPSPawn_BP_C|GetWeaponToEquip _asfpspawn_bp))
  (if (not (== (Variables|/Game/FPSPawn/Blueprints/FPSPawn_BP.FPSPawn_BP_C|GetWeaponEquipped _asfpspawn_bp) _weapontoequip))
    (switch int _weapontoequip
      (:1
        (Variables|/Game/FPSPawn/Blueprints/FPSPawn_BP.FPSPawn_BP_C|SetMain2Weapon _asfpspawn_bp (Utilities|Struct|MakeGunData "NewEnumerator5" "Weapon_AWP_C" (Variables|Default|GetAmmoCnt) (Variables|Default|GetAmmoMax) (Variables|Default|GetReloadTime) (Variables|Default|GetBulletSpread))))
      (:2
        (Variables|/Game/FPSPawn/Blueprints/FPSPawn_BP.FPSPawn_BP_C|SetMain1Weapon _asfpspawn_bp (Utilities|Struct|MakeGunData "NewEnumerator5" "Weapon_AWP_C" (Variables|Default|GetAmmoCnt) (Variables|Default|GetAmmoMax) (Variables|Default|GetReloadTime) (Variables|Default|GetBulletSpread)))))))

(event EventFire
  (bind _returnvalue (Game|GetPlayerCharacter 0))
  (bind _returnvalue_2 (Game|GetPlayerCharacter 0))
  (bind _asfpspawn_bp (Utilities|Casting|CastToFPSPawn_BP _returnvalue))
  (bind _asfpspawn_bp_2 (Utilities|Casting|CastToFPSPawn_BP _returnvalue_2))
  (bind _mesh1p (Variables|/Game/FPSPawn/Blueprints/FPSPawn_BP.FPSPawn_BP_C|GetMesh1P _asfpspawn_bp_2))
  (bind _firstpersoncamera (Variables|/Game/FPSPawn/Blueprints/FPSPawn_BP.FPSPawn_BP_C|GetFirstPersonCamera _asfpspawn_bp))
  (if (not (Variables|/Game/FPSPawn/Blueprints/FPSPawn_BP.FPSPawn_BP_C|GetIsReloading _asfpspawn_bp_2))
    (if (Variables|Default|GetCanFire)
      (if (> (Variables|Default|GetAmmoCnt) 0)
        (Variables|Default|SetCanFire false)
        (Camera|SetFieldOfView (Variables|/Game/FPSPawn/Blueprints/FPSPawn_BP.FPSPawn_BP_C|GetFirstPersonCamera _asfpspawn_bp_2) 9e+01)
        (Transformation|SetRelativeTransform _mesh1p (Math|Transform|MakeTransform "6.400000,5.500000,-23.670000" "0,6.400000, 0" "1,1,1") false false)
        (Rendering|SetVisibility _mesh1p true false)
        (Widget|SetVisibility (Variables|Default|GetScopeHUD) "Hidden")
        (CallFunction|AmmoUpdate)
        (bind (_nozzleloc _impactpoint) (CallFunction|LineTrace))
        (CallFunction|SpawnDecalTracer _nozzleloc _impactpoint _impactpoint)
        (Animation|Montage|PlayMontage (Variables|/Game/FPSPawn/Blueprints/FPSPawn_BP.FPSPawn_BP_C|GetMesh1P _asfpspawn_bp) "/Game/FPSPawn/Animations/Montages/Arms_AWP_Fire_anim_Montage.Arms_AWP_Fire_anim_Montage"
          (:then
            (Utilities|MuzzleFlash)
            (CallFunction|SemoAutoRecoil))
          (:OnBlendOut
            (Variables|Default|SetCanFire true)
            (if (Variables|/Game/FPSPawn/Blueprints/FPSPawn_BP.FPSPawn_BP_C|GetAimDownSight _asfpspawn_bp)
              (Rendering|SetVisibility (Variables|/Game/FPSPawn/Blueprints/FPSPawn_BP.FPSPawn_BP_C|GetGun _asfpspawn_bp) false false)
              (Widget|SetVisibility (Variables|Default|GetScopeHUD) "Visible")
              (Camera|SetFieldOfView _firstpersoncamera (Variables|Default|GetADS_FOV))
              (else
                (Rendering|SetVisibility (Variables|/Game/FPSPawn/Blueprints/FPSPawn_BP.FPSPawn_BP_C|GetMesh1P _asfpspawn_bp) true false)
                (Widget|SetVisibility (Variables|Default|GetScopeHUD) "Hidden")
                (Camera|SetFieldOfView _firstpersoncamera 9e+01)))))
        (else
          (Audio|PlaySound2D "/Game/FPSPawn/Sounds/DryFire.DryFire" 1.0 1.0 0.0 0 0))))))

(event EventADS
  (params (Toggle :type Boolean))
  (bind _returnvalue (Game|GetPlayerCharacter 0))
  (bind _returnvalue_2 (Game|GetPlayerCharacter 0))
  (bind _asfpspawn_bp (Utilities|Casting|CastToFPSPawn_BP _returnvalue_2))
  (bind _asfpspawn_bp_2 (Utilities|Casting|CastToFPSPawn_BP _returnvalue))
  (bind _firstpersoncamera (Variables|/Game/FPSPawn/Blueprints/FPSPawn_BP.FPSPawn_BP_C|GetFirstPersonCamera _asfpspawn_bp))
  (bind _mesh1p (Variables|/Game/FPSPawn/Blueprints/FPSPawn_BP.FPSPawn_BP_C|GetMesh1P _asfpspawn_bp))
  (if (AI|Components|NavMovement|IsFalling (Variables|/Script/Engine.Character|GetCharacterMovement (.AsFPSPawn%20BP (Utilities|Casting|CastToFPSPawn_BP (Game|GetPlayerCharacter 0)))))
    (if Toggle
      (if (Variables|Default|GetCanFire)
        (Rendering|SetVisibility (Variables|/Game/FPSPawn/Blueprints/FPSPawn_BP.FPSPawn_BP_C|GetGun _asfpspawn_bp_2) false false)
        (bind _returnvalue_3 (UserInterface|CreateWidget "/Game/FPSPawn/Blueprints/Weapon/Scope_HUD.Scope_HUD_C"))
        (bind _output_get (Variables|Default|SetScopeHUD _returnvalue_3))
        (UserInterface|Viewport|AddtoViewport _output_get 0)
        (bind _float (Timeline|Timeline_0 Play)
          (:Update
            (Camera|SetFieldOfView _firstpersoncamera (Math|Float|Lerp 9e+01 (Variables|Default|GetADS_FOV) _float))
            (Transformation|SetRelativeTransform _mesh1p (Math|Transform|MakeTransform (Math|Vector|Lerp(Vector) "1.600000,7.800000,-23.677500" "0.000000, 0,-16.500000" _float) "-0.100000, 0, 0" "1,1,1") false false)
            (Variables|Default|SetBulletSpread 5.0))
          (:Finished
            (Rendering|SetVisibility _mesh1p false false))))
      (else
        (Widget|SetVisibility (Variables|Default|GetScopeHUD) "Hidden")
        (Rendering|SetVisibility (Variables|/Game/FPSPawn/Blueprints/FPSPawn_BP.FPSPawn_BP_C|GetMesh1P _asfpspawn_bp_2) true false)
        (bind _float_2 (Timeline|Timeline_1 Play)
          (:Update
            (Camera|SetFieldOfView _firstpersoncamera (Math|Float|Lerp (Variables|Default|GetADS_FOV) 9e+01 _float_2))
            (Transformation|SetRelativeTransform _mesh1p (Math|Transform|MakeTransform (Math|Vector|Lerp(Vector) "0.000000,0.000000,-16.500000" "1.600000,7.800000,-23.677500" _float_2) "0,-6.400000, 0" "1,1,1") false false)
            (Variables|Default|SetBulletSpread 5e+02)))))))

(event EventReload
  (bind _returnvalue (Game|GetPlayerCharacter 0))
  (bind _asfpspawn_bp (Utilities|Casting|CastToFPSPawn_BP _returnvalue))
  (if (< (Variables|Default|GetAmmoCnt) (Variables|Default|GetAmmoMax))
    (Utilities|FlowControl|DoOnce false :!label _label
      (:Completed
        (Variables|/Game/FPSPawn/Blueprints/FPSPawn_BP.FPSPawn_BP_C|SetIsReloading _asfpspawn_bp true)
        (Animation|Montage|MontagePlay (Components|SkeletalMesh|GetAnimInstance (Variables|/Game/FPSPawn/Blueprints/FPSPawn_BP.FPSPawn_BP_C|GetMesh1P _asfpspawn_bp)) "/Game/FPSPawn/Animations/Montages/Arms_AK_Reload_anim_Montage.Arms_AK_Reload_anim_Montage" 1.0 "MontageLength" 0.0 true)
        (Components|Animation|PlayAnimation (Variables|Default|GetPrimaryWeapon) "/Game/FPSPawn/Animations/Montages/AK_Reload_anim_Montage.AK_Reload_anim_Montage" true)
        (Utilities|FlowControl|Delay (Variables|Default|GetReloadTime))
        (Variables|Default|SetAmmoCnt (Variables|Default|GetAmmoMax))
        (Variables|/Game/FPSPawn/Blueprints/FPSPawn_BP.FPSPawn_BP_C|SetIsReloading _asfpspawn_bp false)
        (Variables|Default|SetCanFire true)
        (goto _label Reset)))))

(event EventBeginPlay
  (bind _returnvalue (UserInterface|CreateWidget "/Game/FPSPawn/Blueprints/Weapon/Scope_HUD.Scope_HUD_C"))
  (Variables|Default|SetScopeHUD _returnvalue))

(fn ConstructionScript
  (|CallParentFunction)
  (Variables|Default|SetAmmoMax 10)
  (Variables|Default|SetAmmoCnt 10)
  (Variables|Default|SetReloadTime 3.0)
  (Variables|Default|SetBulletSpread 5.0)
  (Variables|Default|SetRotationOffset "0,-1.100000, 0")
  (Variables|Default|SetName "NewEnumerator5")
  (Variables|Default|SetAutoAvailable false)
  (Variables|Default|SetDamage 99.0)
  (Variables|Default|SetRecoilPitch -1.0)
  (Variables|Default|SetRecoilYaw -0.5)
  (Variables|Default|SetMuzzleFlash 0.5))

(fn AmmoUpdate
  (bind _returnvalue (Math|Random|RandomFloatinRange 0.7 1.2))
  (Math|Integer|DecrementInt (Variables|Default|GetAmmoCnt)
    (:%20%20
      (Audio|PlaySound2D "/Game/FPSPawn/Sounds/Gunshot.Gunshot" (+ _returnvalue -0.2) _returnvalue 0.0 "/Game/FPSPawn/Sounds/Concurrency_AK.Concurrency_AK" 0)
      (Components|Animation|PlayAnimation (Variables|Default|GetPrimaryWeapon) "/Game/FPSPawn/Animations/Weapons/AK_Fire_anim.AK_Fire_anim" false))))

(fn LineTrace
  (bind _returnvalue (Game|GetPlayerCharacter 0))
  (bind _bulletspread (Variables|Default|GetBulletSpread))
  (bind _muzzle (Variables|Default|GetMuzzle))
  (bind _returnvalue_2 (Transformation|GetWorldLocation _muzzle))
  (bind _returnvalue_3 (* _bulletspread -1.0))
  (bind _asfpspawn_bp (Utilities|Casting|CastToFPSPawn_BP _returnvalue))
  (bind _firstpersoncamera (Variables|/Game/FPSPawn/Blueprints/FPSPawn_BP.FPSPawn_BP_C|GetFirstPersonCamera _asfpspawn_bp))
  (bind _returnvalue_4 (Transformation|GetWorldLocation _firstpersoncamera))
  (bind _outhit (Collision|LineTraceByChannel (+ _returnvalue_4 (Variables|Default|GetAimOffset)) (+ (+ _returnvalue_4 (* (Math|Vector|GetForwardVector _firstpersoncamera) 2e+04)) (Math|Vector|MakeVector (Math|Random|RandomFloatinRange _returnvalue_3 _bulletspread) (Math|Random|RandomFloatinRange _returnvalue_3 _bulletspread) (Math|Random|RandomFloatinRange _returnvalue_3 _bulletspread))) "TraceTypeQuery1" false 0 "None")) ; CameraShot
  (Collision|LineTraceByChannel _returnvalue_2 (.ImpactPoint (Collision|BreakHitResult _outhit)) "TraceTypeQuery1" false 0 "None" true "(R=0.160040,G=1.000000,B=0.000000,A=1.000000)") ; GunShot
  (if (.bSuccess (Utilities|Casting|CastToAIPawn_BP (.HitActor (Collision|BreakHitResult _outhit))))
    (Default|Jahae (.AsAIPawn%20BP (Utilities|Casting|CastToAIPawn_BP (.HitActor (Collision|BreakHitResult _outhit))))))
  (return _returnvalue_2 (.ImpactPoint (Collision|BreakHitResult _outhit))))

(fn SpawnDecalTracer
  (params (Location :type Vector) (SpawnTransformLoc :type Vector) (ImpactPoint :type Vector))
  (Game|SpawnActorfromClass "/Game/FPSPawn/Animations/Montages/BulletDecal_BP.BulletDecal_BP_C" (Math|Transform|MakeTransform SpawnTransformLoc (Math|Conversions|RotationFromXVector ImpactPoint) "0.250000,0.250000,0.250000") "Undefined" 0 0)
  (if (>= (Math|Random|RandomIntegerinRange 1 10) 5)
    (Game|SpawnActorfromClass "/Game/FPSPawn/Blueprints/Weapon/TracerRound_BP.TracerRound_BP_C" (Math|Transform|MakeTransform Location (Transformation|GetWorldRotation (Variables|/Game/FPSPawn/Blueprints/FPSPawn_BP.FPSPawn_BP_C|GetFirstPersonCamera (.AsFPSPawn%20BP (Utilities|Casting|CastToFPSPawn_BP (Game|GetPlayerCharacter 0))))) "0.050000,0.050000,0.050000") "Undefined" 0 0))
  (return))

(fn SemoAutoRecoil
  (bind _returnvalue (Game|GetPlayerController 0))
  (bind _recoilpitch (Variables|Default|GetRecoilPitch))
  (bind _recoilyaw (Variables|Default|GetRecoilYaw))
  (Class|PlayerController|AddPitchInput _returnvalue (Math|Random|RandomFloatinRange (* 1.5 _recoilpitch) _recoilpitch))
  (Class|PlayerController|AddYawInput _returnvalue (Math|Random|RandomFloatinRange _recoilyaw (* -1.0 _recoilyaw))))