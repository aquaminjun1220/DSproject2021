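; Extraction zone actor that shows the player's score once the FPS pawn has waited inside it for a few seconds.
; Entering clears the Out flag, adds a waiting-for-extraction widget and starts a retriggerable delay, which re-entry restarts.
; Leaving sets Out and removes the widget, so the pending delay finishes without effect.
; If Out is still false when the delay ends, it calls DisplayScore on the player character.
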(event Collision|EventActorBeginOverlap
  (params (OtherActor :type Actor%20Object%20Reference))
  (Utilities|Casting|CastToFPSPawn_BP OtherActor)
  (Variables|Default|SetOut? false)
  (bind _returnvalue (UserInterface|CreateWidget "/Game/Blueprints/Menu/ExtractionMenu/waitingForExtractionUMG.waitingForExtractionUMG_C" (Game|GetPlayerController 0)))
  (bind _output_get (Variables|Default|SetExtraction%20UMG _returnvalue))
  (UserInterface|Viewport|AddtoViewport _output_get 0)
  (Utilities|FlowControl|RetriggerableDelay 5.0)
  (if (not (Variables|Default|GetOut?))
    (Default|DisplayScore (.AsFPSPawn%20BP (Utilities|Casting|CastToFPSPawn_BP (Game|GetPlayerCharacter 0))))))

(event Collision|EventActorEndOverlap
  (params (OtherActor :type Actor%20Object%20Reference))
  (Utilities|Casting|CastToFPSPawn_BP OtherActor)
  (Variables|Default|SetOut? true)
  (Widget|RemovefromParent (Variables|Default|GetExtraction%20UMG)))

(fn ConstructionScript)