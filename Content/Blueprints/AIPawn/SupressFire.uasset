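; Behavior tree task that makes an AI pawn lay down suppressing fire toward its blackboard target.
; It turns the pawn's yaw toward the stored target location, keeping pitch and roll, then calls the pawn's Fire.
; A small weighted random chance also calls Jahae on the target FPS pawn.
; The task finishes successfully in the same execution, though a failed cast leaves it unfinished.
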(event EventReceiveExecuteAI
  (params (OwnerController :type AI%20Controller%20Object%20Reference) (ControlledPawn :type Pawn%20Object%20Reference))
  (bind _asaipawn_bp (Utilities|Casting|CastToAIPawn_BP ControlledPawn))
  (Variables|Default|SetAIPawn _asaipawn_bp)
  (Transformation|SetActorRotation ControlledPawn (Math|Rotator|MakeRotator (.roll (Transformation|GetActorRotation (Variables|Default|GetAIPawn))) (.pitch (Transformation|GetActorRotation (Variables|Default|GetAIPawn))) (.yaw (Math|Rotator|FindLookatRotation (Transformation|GetActorLocation (Variables|Default|GetAIPawn)) (Class|BTFunctionLibrary|GetBlackboardValueasVector (Variables|Default|GetTargetActorLocation))))))
  (Default|Fire (Variables|Default|GetAIPawn))
  (if (Math|Random|RandomBoolwithWeight 0.02)
    (bind _asfpspawn_bp (Utilities|Casting|CastToFPSPawn_BP (AI|BehaviorTree|GetBlackboardValueasActor (Variables|Default|GetTargetActor))))
    (Default|Jahae _asfpspawn_bp))
  (AI|BehaviorTree|FinishExecute true))