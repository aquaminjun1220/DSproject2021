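; AI controller for the basic AI pawn that runs its behavior tree and feeds target information into the blackboard.
; It starts AI_basic_BT on BeginPlay.
; Perception updates set TargetActor to the sensed actor, or clear it when sensing fails.
; An onHit event stores player pawn 0 in TargetActorMemory, regardless of who caused the hit.
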(event OnTargetPerceptionUpdated(AIPerception)
  (params (Actor :type Actor%20Object%20Reference) (Stimulus :type AI%20Stimulus%20Structure))
  (if (.bSuccessfullySensed (Utilities|Struct|BreakAIStimulus Stimulus))
    (AI|Components|Blackboard|SetValueasObject (Variables|Default|GetBlackboard) (Utilities|Name|MakeLiteralName "TargetActor") Actor)
    (else
      (AI|Components|Blackboard|SetValueasObject (Variables|Default|GetBlackboard) (Utilities|Name|MakeLiteralName "TargetActor") 0))))

(event Custom|onHit
  (AI|Components|Blackboard|SetValueasObject (Variables|Default|GetBlackboard) (Utilities|Name|MakeLiteralName "TargetActorMemory") (Game|Player|GetPlayerPawn 0)))

(event EventBeginPlay
  (AI|RunBehaviorTree "/Game/Blueprints/AIPawn/AI_basic/AI_basic_BT.AI_basic_BT"))

(fn ConstructionScript)