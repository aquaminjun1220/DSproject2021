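; AI enemy pawn with health, a floating health bar and gunfire effects, which awards score to the player on death.
; Fire plays a gunshot and briefly flashes a point light and muzzle mesh, then randomizes the mesh's pitch and scale.
; Jahae applies damage, notifies AI_basic_ContBP and shows the health bar until a one-second retriggerable delay expires.
; Lethal damage calls Die, adding AIScore to FPSPawn_BP before destroying the actor.
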(event Custom|Fire
  (bind _returnvalue (Math|Random|RandomFloatinRange 0.4 1.2))
  (bind _staticmesh (Variables|Default|GetStaticMesh))
  (Audio|PlaySoundatLocation "/Game/Assets/Sounds/FPSPawn/Gunshot.Gunshot" (Transformation|GetWorldLocation (Variables|Default|GetPointLight)) "0, 0, 0" 0.5 1.0 0.0 "/Game/Assets/Sounds/FPSPawn/Attenuation_AK.Attenuation_AK" "/Game/Assets/Sounds/FPSPawn/Concurrency_AK.Concurrency_AK" 0)
  (Rendering|Components|Light|SetIntensity (Variables|Default|GetPointLight) 2e+04)
  (Rendering|SetVisibility (Variables|Default|GetStaticMesh) true false)
  (Utilities|FlowControl|Delay 0.07)
  (Rendering|Components|Light|SetIntensity (Variables|Default|GetPointLight) 0.0)
  (Rendering|SetVisibility _staticmesh false false)
  (Transformation|SetRelativeRotation _staticmesh (Math|Rotator|MakeRotator 9e+01 (Math|Random|RandomFloatinRange -9e+01 9e+01) 9e+01) false false)
  (Transformation|SetWorldScale3D _staticmesh (Math|Vector|MakeVector _returnvalue _returnvalue _returnvalue)))

(event Custom|Jahae
  (params (dmg :type Float%20%28single-precision%29))
  (bind _asai_basic_cont_bp (Utilities|Casting|CastToAI_basic_ContBP (Pawn|GetController)))
  (Default|OnHit _asai_basic_cont_bp)
  (if (> (Math|Conversions|ToFloat(Integer) (Variables|Default|GetHealth)) dmg)
    (Variables|Default|SetHealth (Math|Float|Truncate (- (Math|Conversions|ToFloat(Integer) (Variables|Default|GetHealth)) dmg)))
    (Variables|/Game/Blueprints/AIPawn/AIHealth.AIHealth_C|SetHPpercent (Variables|Default|GetAIHealth) (/ (Math|Conversions|ToFloat(Integer) (Variables|Default|GetHealth)) (Variables|Default|GetMaxHealth)))
    (Widget|SetRenderOpacity (Variables|Default|GetAIHealth) 1.0)
    (Utilities|FlowControl|RetriggerableDelay 1.0)
    (Widget|SetRenderOpacity (Variables|Default|GetAIHealth) 0.0)
    (else
      (CallFunction|Die))))

(event Custom|Die
  (bind _returnvalue (Game|GetPlayerCharacter 0))
  (bind _asfpspawn_bp (Utilities|Casting|CastToFPSPawn_BP _returnvalue))
  (Variables|/Game/Blueprints/FPSPawn/FPSPawn_BP.FPSPawn_BP_C|SetScore _asfpspawn_bp (+ (Variables|/Game/Blueprints/FPSPawn/FPSPawn_BP.FPSPawn_BP_C|GetScore _asfpspawn_bp) (Variables|Default|GetAI_score)))
  (Actor|DestroyActor))

(event EventBeginPlay
  (bind _asaihealth (Utilities|Casting|CastToAIHealth (UserInterface|GetUserWidgetObject (Variables|Default|GetHPBar))))
  (bind _output_get (Variables|Default|SetAIHealth _asaihealth))
  (Variables|/Game/Blueprints/AIPawn/AIHealth.AIHealth_C|SetHPpercent _output_get (/ (Math|Conversions|ToFloat(Integer) (Variables|Default|GetHealth)) (Variables|Default|GetMaxHealth)))
  (Widget|SetRenderOpacity _output_get 0.0))

(fn ConstructionScript)