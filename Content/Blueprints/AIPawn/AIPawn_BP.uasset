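; AI pawn Blueprint that provides gunfire effects and simple health-based damage.
; Fire plays an attenuated, concurrency-limited gunshot and briefly flashes a point light and muzzle mesh.
; After hiding the mesh, it randomizes rotation and scale so the next flash looks different.
; Jahae subtracts damage from integer Health, truncating the result, and destroys the actor when damage meets or exceeds Health.
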(event Custom|Fire
  (bind _returnvalue (Math|Random|RandomFloatinRange 0.4 1.2))
  (bind _staticmesh (Variables|Default|GetStaticMesh))
  (Audio|PlaySoundatLocation "/Game/Assets/Sounds/FPSPawn/Gunshot.Gunshot" (Transformation|GetWorldLocation (Variables|Default|GetPointLight)) "0, 0, 0" 0.5 1.0 0.0 "/Game/Assets/Sounds/FPSPawn/Attenuation_AK.Attenuation_AK" "/Game/Assets/Sounds/FPSPawn/Concurrency_AK.Concurrency_AK" 0)
  (Rendering|Components|Light|SetIntensity (Variables|Default|GetPointLight) 2e+04)
  (Rendering|SetVisibility (Variables|Default|GetStaticMesh) true false)
  (Utilities|FlowControl|Delay 0.07)
  (Rendering|Components|Light|SetIntensity (Variables|Default|GetPointLight) 0.0)
  (Rendering|SetVisibility _staticmesh false false)
  (Transformation|SetRelativeRotation _staticmesh (Math|Rotator|MakeRotator 9e+01 (Math|Random|RandomFloatinRange -9e+01 9e+01) 9e+01) false false)
  (Transformation|SetWorldScale3D _staticmesh (Math|Vector|MakeVector _returnvalue _returnvalue _returnvalue)))

(event Custom|Jahae
  (params (dmg :type Float%20%28single-precision%29))
  (if (> (Math|Conversions|ToFloat(Integer) (Variables|Default|GetHealth)) dmg)
    (Variables|Default|SetHealth (Math|Float|Truncate (- (Math|Conversions|ToFloat(Integer) (Variables|Default|GetHealth)) dmg)))
    (else
      (Actor|DestroyActor))))

(fn ConstructionScript)