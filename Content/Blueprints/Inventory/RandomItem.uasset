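; RandomItem is a placeholder actor that randomly replaces itself with an item (Goosang, WaterBottle or CupRamen) or with nothing.
; On BeginPlay it takes one random roll and tests it against non-overlapping probability bands through SpawnRandomItem, leaving a 70% chance of no spawn.
; A matching class spawns at the actor's location, adjusted for collisions but always spawned, and the placeholder then destroys itself.
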(event EventBeginPlay
  (Variables|Default|SetProb (Math|Random|RandomFloat))
  (Utilities|SpawnRandomItem 0.0 0.05 "/Game/Blueprints/Inventory/goosang.goosang_C")
  (Utilities|SpawnRandomItem 0.05 0.2 "/Game/Blueprints/Inventory/WaterBottle.WaterBottle_C")
  (Utilities|SpawnRandomItem 0.2 0.3 "/Game/Blueprints/Inventory/CupRamen.CupRamen_C")
  (Actor|DestroyActor))

(fn ConstructionScript)