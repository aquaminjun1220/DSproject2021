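; RandomWeapon is a placeable spawner actor that randomly leaves a weapon pickup at its location, or usually nothing.
; On BeginPlay it rolls one float from 0 to 2 and passes adjacent narrow bands to SpawnRandomItem for the AWP, AK, Glock and MP5 pickups.
; The bands cover only up to 0.14, so about 7% of rolls spawn a weapon.
; The spawner then destroys itself either way.
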(event EventBeginPlay
  (Variables|Default|SetProb (Math|Random|RandomFloatinRange 0.0 2.0))
  (Utilities|SpawnRandomItem 0.0 0.02 "/Game/Blueprints/FPSPawn/Weapon/PickUp_AWP.PickUp_AWP_C")
  (Utilities|SpawnRandomItem 0.02 0.05 "/Game/Blueprints/FPSPawn/Weapon/PickUp_AK.PickUp_AK_C")
  (Utilities|SpawnRandomItem 0.05 0.1 "/Game/Blueprints/FPSPawn/Weapon/PickUp_Glock.PickUp_Glock_C")
  (Utilities|SpawnRandomItem 0.1 0.14 "/Game/Blueprints/FPSPawn/Weapon/PickUp_MP5.PickUp_MP5_C")
  (Actor|DestroyActor))

(fn ConstructionScript)