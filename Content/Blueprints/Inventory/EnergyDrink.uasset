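; EnergyDrink is an inventory item Blueprint that restores player stamina when used.
; Its ItemUse event casts player character 0 to FPSPawn_BP and adds a fixed amount to Stamina, clamped to a maximum with Min.
; BeginPlay, overlap and Tick are disabled stubs, and the construction script only calls its parent.
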(event EventBeginPlay
  (|CallParentFunction) ; This node is disabled and will not be called.\nDrag off pins to build functionality.
)

(event Collision|EventActorBeginOverlap
  (params (OtherActor :type Actor%20Object%20Reference))
  (|CallParentFunction OtherActor) ; This node is disabled and will not be called.\nDrag off pins to build functionality.
)

(event EventTick
  (params (DeltaSeconds :type Float%20%28single-precision%29))
  (|CallParentFunction DeltaSeconds) ; This node is disabled and will not be called.\nDrag off pins to build functionality.
)

(event EventItemUse
  (bind _returnvalue (Game|GetPlayerCharacter 0))
  (bind _asfpspawn_bp (Utilities|Casting|CastToFPSPawn_BP _returnvalue))
  (Variables|/Game/Blueprints/FPSPawn/FPSPawn_BP.FPSPawn_BP_C|SetStamina _asfpspawn_bp (Math|Float|Min(Float) (+ (Variables|/Game/Blueprints/FPSPawn/FPSPawn_BP.FPSPawn_BP_C|GetStamina _asfpspawn_bp) 6e+01) 1e+02)))

(fn ConstructionScript
  (|CallParentFunction))