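; AI pawn Blueprint that handles gunfire effects and a simple health-based death.
; Fire plays an attenuated gunshot and briefly flashes a point light and static mesh, then randomizes the mesh's pitch and scale for the next shot.
; Jahae subtracts a fixed amount of Health per call, destroying the actor only on a call where Health is already below zero.
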(event Custom|Fire
  (bind _returnvalue (Math|Random|RandomFloatinRange 0.4 1.2))
  (bind _staticmesh (Variables|Default|GetStaticMesh))
  (Audio|PlaySoundatLocation "/Game/FPSPawn/Sounds/Gunshot.Gunshot" (Transformation|GetWorldLocation (Variables|Default|GetPointLight)) "0, 0, 0" 0.5 1.0 0.0 "/Game/FPSPawn/Sounds/Attenuation_AK.Attenuation_AK" "/Game/FPSPawn/Sounds/Concurrency_AK.Concurrency_AK" 0)
  (Rendering|Components|Light|SetIntensity (Variables|Default|GetPointLight) 2e+04)
  (Rendering|SetVisibility (Variables|Default|GetStaticMesh) true false)
  (Utilities|FlowControl|Delay 0.07)
  (Rendering|Components|Light|SetIntensity (Variables|Default|GetPointLight) 0.0)
  (Rendering|SetVisibility _staticmesh false false)
  (Transformation|SetRelativeRotation _staticmesh (Math|Rotator|MakeRotator 9e+01 (Math|Random|RandomFloatinRange -9e+01 9e+01) 9e+01) false false)
  (Transformation|SetWorldScale3D _staticmesh (Math|Vector|MakeVector _returnvalue _returnvalue _returnvalue)))

(event Custom|Jahae
  (if (< (Variables|Default|GetHealth) 0)
    (Actor|DestroyActor)
    (else
      (Variables|Default|SetHealth (- (Variables|Default|GetHealth) 9)))))

(fn ConstructionScript)